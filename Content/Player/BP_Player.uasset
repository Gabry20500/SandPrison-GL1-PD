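; Player actor for a turn-based grid battle, with health, AP and attacks on enemy cells.
; WASD or arrow keys step it through a bounded grid with a cooldown, mapping grid positions to transforms via GridRef and sliding with MoveComponentTo.
; BaseAttack, Mutilation and Subjugation damage enemies from the GameManager's list; Subjugation affects all, regardless of cell.
; Poses are material swaps reset after delays, and death quits the game.
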(event Custom|UpdateGridTransform
  ;[1 1 1] Event to set the current Transform using current grid pos(We need an event because MoveComponentTo function is reachable only from EventGraph)
  (Rendering|Material|SetMaterial (Variables|Default|GetMesh) 0 "/Game/Player/Pose/DodgePose/DodgePoseMat_Inst.DodgePoseMat_Inst")
  (for _array_element (Variables|Default|GetGridRef)
    (for _index (range 0 (- (Utilities|Array|Length (.gridposition _array_element)) 1))
      (if (Math|Vector|Equal(Vector) (Variables|Default|GetCurrentGridPos) (Utilities|Array|Get(acopy) (.gridposition _array_element) _index) 0.1)
        (Components|MoveComponentTo (Variables|Default|GetDefaultSceneRoot) (Utilities|Array|Get(acopy) (.gridtransform _array_element) _index) (Transformation|GetWorldRotation (Variables|Default|GetDefaultSceneRoot)) false false 0.3 false)
        (CallFunction|SetIdleMeshforDodge)))))

(event Custom|SetIdleMeshForDodge
  (Utilities|FlowControl|Delay 0.2)
  (Rendering|Material|SetMaterial (Variables|Default|GetMesh) 0 "/Game/Player/Pose/IdlePose/idle_pose_Mat_Inst.idle_pose_Mat_Inst"))

(event Custom|SetIdleMesh
  (Utilities|FlowControl|Delay 0.5)
  (Rendering|Material|SetMaterial (Variables|Default|GetMesh) 0 "/Game/Player/Pose/IdlePose/idle_pose_Mat_Inst.idle_pose_Mat_Inst"))

(event EventBeginPlay
  ;[1 1 1] Set CurrentGridPos by checking current transform
  (CallFunction|UpdateGridPos)
  (bind _returnvalue (Actor|GetActorOfClass "/Game/BP_GameManager.BP_GameManager_C"))
  (Variables|Default|SetGMref _returnvalue))

(event EventTick
  (params (DeltaSeconds :type Float%20%28single-precision%29))
  (Development|PrintString (Utilities|String|ToString(Boolean) (Variables|Default|GetIsMyTurn?)) true true "(R=0.000000,G=0.660000,B=1.000000,A=1.000000)" 0.0)
  (Variables|Default|SetPlayerLocation (Transformation|GetWorldLocation (Variables|Default|GetMesh))))

(event Input|KeyboardEvents|Right
  (params (Key :type Key%20Structure))
  ;[1 1 1] Moving Right/Left, calling key event and checking axis value
  (:Pressed
    (if (Variables|Default|GetCanMove)
      (Variables|Default|SetCanMove false)
      (CallFunction|MoveRightLeft)
      (if (not (Variables|Default|GetCanMove))
        (Utilities|FlowControl|Delay 0.4)
        (Variables|Default|SetCanMove true)))))

(event Input|KeyboardEvents|D
  (params (Key :type Key%20Structure))
  ;[1 1 1] Moving Right/Left, calling key event and checking axis value
  (:Pressed
    (if (Variables|Default|GetCanMove)
      (Variables|Default|SetCanMove false)
      (CallFunction|MoveRightLeft)
      (if (not (Variables|Default|GetCanMove))
        (Utilities|FlowControl|Delay 0.4)
        (Variables|Default|SetCanMove true)))))

(event Input|KeyboardEvents|Down
  (params (Key :type Key%20Structure))
  ;[1 1 1] Moving UP/DOWN, calling key event and checking axis value
  (:Pressed
    (if (Variables|Default|GetCanMove)
      (Variables|Default|SetCanMove false)
      (CallFunction|MoveUpDown)
      (if (not (Variables|Default|GetCanMove))
        (Utilities|FlowControl|Delay 0.4)
        (Variables|Default|SetCanMove true)))))

(event Input|KeyboardEvents|S
  (params (Key :type Key%20Structure))
  ;[1 1 1] Moving UP/DOWN, calling key event and checking axis value
  (:Pressed
    (if (Variables|Default|GetCanMove)
      (Variables|Default|SetCanMove false)
      (CallFunction|MoveUpDown)
      (if (not (Variables|Default|GetCanMove))
        (Utilities|FlowControl|Delay 0.4)
        (Variables|Default|SetCanMove true)))))

(event Input|KeyboardEvents|W
  (params (Key :type Key%20Structure))
  ;[1 1 1] Moving UP/DOWN, calling key event and checking axis value
  (:Pressed
    (if (Variables|Default|GetCanMove)
      (Variables|Default|SetCanMove false)
      (CallFunction|MoveUpDown)
      (if (not (Variables|Default|GetCanMove))
        (Utilities|FlowControl|Delay 0.4)
        (Variables|Default|SetCanMove true)))))

(event Input|KeyboardEvents|Up
  (params (Key :type Key%20Structure))
  ;[1 1 1] Moving UP/DOWN, calling key event and checking axis value
  (:Pressed
    (if (Variables|Default|GetCanMove)
      (Variables|Default|SetCanMove false)
      (CallFunction|MoveUpDown)
      (if (not (Variables|Default|GetCanMove))
        (Utilities|FlowControl|Delay 0.4)
        (Variables|Default|SetCanMove true)))))

(event Input|KeyboardEvents|A
  (params (Key :type Key%20Structure))
  ;[1 1 1] Moving Right/Left, calling key event and checking axis value
  (:Pressed
    (if (Variables|Default|GetCanMove)
      (Variables|Default|SetCanMove false)
      (CallFunction|MoveRightLeft)
      (if (not (Variables|Default|GetCanMove))
        (Utilities|FlowControl|Delay 0.4)
        (Variables|Default|SetCanMove true)))))

(event Input|KeyboardEvents|Left
  (params (Key :type Key%20Structure))
  ;[1 1 1] Moving Right/Left, calling key event and checking axis value
  (:Pressed
    (if (Variables|Default|GetCanMove)
      (Variables|Default|SetCanMove false)
      (CallFunction|MoveRightLeft)
      (if (not (Variables|Default|GetCanMove))
        (Utilities|FlowControl|Delay 0.4)
        (Variables|Default|SetCanMove true)))))

(fn ConstructionScript)

(fn UpdateGridPos
  (bind _mesh (Variables|Default|GetMesh))
  (bind _returnvalue (Transformation|GetWorldLocation _mesh))
  (for _array_element (Variables|Default|GetGridRef)
    (for _index (range 0 (- (Utilities|Array|Length (.gridtransform _array_element)) 1))
      (if (Math|Vector|Equal(Vector) (Math|Vector|MakeVector (.x _returnvalue) (.y _returnvalue) 0.0) (Math|Vector|MakeVector (.x (Utilities|Array|Get(acopy) (.gridtransform _array_element) _index)) (.y (Utilities|Array|Get(acopy) (.gridtransform _array_element) _index)) 0.0) 3e+01)
        (bind _output_get (Variables|Default|SetCurrentGridPos (Utilities|Array|Get(acopy) (.gridposition _array_element) _index)))
        (return _output_get)))))

(fn MoveUpDown
  (switch int (Math|Float|Truncate (Input|AxisValues|GetMoveForward))
    (:-1
      (if (== (.y (Variables|Default|GetCurrentGridPos)) -2.0)
        (Variables|Default|SetCanMove true)
        (else
          (Variables|Default|SetCurrentGridPos (Math|Vector2D|MakeVector2D (.x (Variables|Default|GetCurrentGridPos)) (- (.y (Variables|Default|GetCurrentGridPos)) 1.0)))
          ;[1 1 1] Set current world Transform upon current gridPos
          (CallFunction|UpdateGridTransform :!label _label))))
    (:1
      (if (== (.y (Variables|Default|GetCurrentGridPos)) 2.0)
        (Variables|Default|SetCanMove true)
        (else
          (Variables|Default|SetCurrentGridPos (Math|Vector2D|MakeVector2D (.x (Variables|Default|GetCurrentGridPos)) (+ (.y (Variables|Default|GetCurrentGridPos)) 1.0)))
          (goto _label))))))

(fn MoveRightLeft
  (switch int (Math|Float|Truncate (Input|AxisValues|GetMoveSide))
    (:-1
      (if (== (.x (Variables|Default|GetCurrentGridPos)) -4.0)
        (Variables|Default|SetCanMove true)
        (else
          (Variables|Default|SetCurrentGridPos (Math|Vector2D|MakeVector2D (- (.x (Variables|Default|GetCurrentGridPos)) 1.0) (.y (Variables|Default|GetCurrentGridPos))))
          ;[1 1 1] Set current world Transform upon current gridPos
          (CallFunction|UpdateGridTransform :!label _label))))
    (:1
      (if (== (.x (Variables|Default|GetCurrentGridPos)) 0.0)
        (Variables|Default|SetCanMove true)
        (else
          (Variables|Default|SetCurrentGridPos (Math|Vector2D|MakeVector2D (+ (.x (Variables|Default|GetCurrentGridPos)) 1.0) (.y (Variables|Default|GetCurrentGridPos))))
          (goto _label))))))

(fn BaseAttack
  (params (AttackLocation :type Integer))
  ;[1 1 1] Base Attack
  (LocalVariables|SetCellSelected (Utilities|Array|Get(acopy) (.gridposition (Variables|Default|GetEnemyGrid)) AttackLocation))
  (for _array_element (Variables|/Game/BP_GameManager.BP_GameManager_C|GetEnemyList (Variables|Default|GetGMref))
    (if (Math|Vector|Equal(Vector) (Variables|/Game/Enemies/BP_Enemy.BP_Enemy_C|GetMyGridPos _array_element) (LocalVariables|GetCellSelected) 0.0001)
      (Default|TakeDamage _array_element 2e+01)
      (Variables|Default|SetImDone true)
      (Rendering|Material|SetMaterial (Variables|Default|GetMesh) 0 "/Game/Player/Pose/BaseAttack/BaseAttack_Mat_Inst.BaseAttack_Mat_Inst")
      (CallFunction|SetIdleMesh))))

(fn EndMyTurn
  (Variables|Default|SetIsMyTurn? false)
  (bind _returnvalue (UserInterface|CreateWidget "/Game/Player/UI/Attack_UI/BaseAttack_UI_WG.BaseAttack_UI_WG_C"))
  (Default|SetHidden _returnvalue))

(fn TakeDamage
  (params (DMG :type Float%20%28single-precision%29))
  (bind _output_get (Variables|Default|SetHealth (- (Variables|Default|GetHealth) DMG)))
  (if (<= _output_get 0.0)
    (Game|QuitGame 0 "Quit" false)))

(fn BeginTurn
  (Variables|Default|SetIsMyTurn? true)
  (Variables|Default|SetImDone false)
  (UserInterface|CreateWidget "/Game/Player/UI/Attack_UI/BaseAttack_UI_WG.BaseAttack_UI_WG_C"))

(fn Mutilation
  (params (Attack%20location :type Integer))
  (LocalVariables|SetCellSelected (Utilities|Array|Get(acopy) (.gridposition (Variables|Default|GetEnemyGrid)) Attack%20location))
  (Variables|Default|SetAP (- (Variables|Default|GetAP) 2))
  (for _array_element (Variables|/Game/BP_GameManager.BP_GameManager_C|GetEnemyList (Variables|Default|GetGMref))
    (Variables|Default|SetArray%20Element _array_element)
    (if (Math|Vector|Equal(Vector) (Variables|/Game/Enemies/BP_Enemy.BP_Enemy_C|GetMyGridPos _array_element) (LocalVariables|GetCellSelected) 0.0001)
      (Rendering|Material|SetMaterial (Variables|Default|GetMesh) 0 "/Game/Player/Pose/MutilationPose/MutilationMat_Inst.MutilationMat_Inst")
      (if (== (Variables|/Game/Enemies/BP_Enemy.BP_Enemy_C|GetHealth (Variables|Default|GetArray%20Element)) (Variables|/Game/Enemies/BP_Enemy.BP_Enemy_C|GetMaxHP (Variables|Default|GetArray%20Element)))
        (Default|TakeDamage (Variables|Default|GetArray%20Element) (* 20 2.5))
        (Variables|Default|SetImDone true)
        (else
          (Default|TakeDamage (Variables|Default|GetArray%20Element) 2e+01)
          (Variables|Default|SetImDone true)))
      (CallFunction|SetIdleMesh))))

(fn AddAp
  (params (ValueToAdd :type Integer))
  (Variables|Default|SetAP (+ ValueToAdd (Variables|Default|GetAP)))
  (if (> (Variables|Default|GetAP) 0)
    (Variables|Default|SetAP 10)))

(fn Subjugation
  (params (Attack%20location :type Integer))
  (LocalVariables|SetCellSelected (Utilities|Array|Get(acopy) (.gridposition (Variables|Default|GetEnemyGrid)) Attack%20location))
  (Variables|Default|SetAP (- (Variables|Default|GetAP) 3))
  (for _array_element (Variables|/Game/BP_GameManager.BP_GameManager_C|GetEnemyList (Variables|Default|GetGMref))
    (bind _output_get (Variables|Default|SetArray%20Element _array_element))
    (if (Math|Vector|Equal(Vector) (Variables|/Game/Enemies/BP_Enemy.BP_Enemy_C|GetMyGridPos _array_element) (LocalVariables|GetCellSelected) 0.0001)
      _
      (else
        _))
    (Variables|/Game/Enemies/BP_Enemy.BP_Enemy_C|SetisVulnerable _output_get true)
    (Rendering|Material|SetMaterial (Variables|Default|GetMesh) 0 "/Game/Player/Pose/SubjugationPose/SubjugationPosemat_Inst.SubjugationPosemat_Inst")
    (Variables|Default|SetImDone true)
    (Default|TakeDamage (Variables|Default|GetArray%20Element) (* 20 2.0))
    (CallFunction|SetIdleMesh)))