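; BP_Grid is a grid actor that toggles selection highlights for three attacks: BaseAttack, Mutilation and Subjugation.
; Each attack has Add and Remove events that show or hide its component.
; Adding BaseAttack or Mutilation hides the other two and disables their collision, and removing any selection restores QueryOnly collision on the others.
; Adding Subjugation only changes visibility, as its collision-disabling nodes are never run.
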(event Custom|RemoveSelectionGridsk2
  ;[1 1 1] Subjugation
  (Rendering|SetVisibility (Variables|Default|GetSubjugation) false false)
  (Collision|SetCollisionEnabled (Variables|Default|GetBase%20Attack) "QueryOnly")
  (Collision|SetCollisionEnabled (Variables|Default|GetMutilation) "QueryOnly"))

(event Custom|AddSelectionGridBA
  ;[1 1 1] Base attack
  (Rendering|SetVisibility (Variables|Default|GetBase%20Attack) true false)
  (Rendering|SetVisibility (Variables|Default|GetMutilation) false false)
  (Rendering|SetVisibility (Variables|Default|GetSubjugation) false false)
  (Collision|SetCollisionEnabled (Variables|Default|GetMutilation) "NoCollision")
  (Collision|SetCollisionEnabled (Variables|Default|GetSubjugation) "NoCollision"))

(event Custom|RemoveSelectionGridBA
  ;[1 1 1] Base attack
  (Rendering|SetVisibility (Variables|Default|GetBase%20Attack) false false)
  (Collision|SetCollisionEnabled (Variables|Default|GetMutilation) "QueryOnly")
  (Collision|SetCollisionEnabled (Variables|Default|GetSubjugation) "QueryOnly"))

(event Custom|AddSelectionGridsk2
  ;[1 1 1] Subjugation
  (Rendering|SetVisibility (Variables|Default|GetSubjugation) true false)
  (Rendering|SetVisibility (Variables|Default|GetBase%20Attack) false false)
  (Rendering|SetVisibility (Variables|Default|GetMutilation) false false))

(event Custom|RemoveSelectionGridSk1
  ;[1 1 1] Mutilation
  (Rendering|SetVisibility (Variables|Default|GetMutilation) false false)
  (Collision|SetCollisionEnabled (Variables|Default|GetBase%20Attack) "QueryOnly")
  (Collision|SetCollisionEnabled (Variables|Default|GetSubjugation) "QueryOnly"))

(event Custom|AddSelectionGridSk1
  ;[1 1 1] Mutilation
  (Rendering|SetVisibility (Variables|Default|GetMutilation) true false)
  (Rendering|SetVisibility (Variables|Default|GetBase%20Attack) false false)
  (Rendering|SetVisibility (Variables|Default|GetSubjugation) false false)
  (Collision|SetCollisionEnabled (Variables|Default|GetBase%20Attack) "NoCollision")
  (Collision|SetCollisionEnabled (Variables|Default|GetSubjugation) "NoCollision"))

(fn ConstructionScript)