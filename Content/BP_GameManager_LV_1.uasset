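; Level 1 game manager that runs turn-based combat between the spawned player and grid-based Brawler enemies.
; BeginPlay spawns the player, then places Brawlers on random cells, re-rolling occupied ones.
; A timeline times the player's turn until they finish or time expires, then enemies attack sequentially with delays before occupied positions refresh and the loop restarts.
; A helper function rebuilds the enemy list, excluding dying enemies.
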(event Custom|LoopStart
  (bind _playerref (Variables|Default|GetPlayerRef))
  (for _index (range 0 99) :!label _label
    (Default|BeginTurn _playerref)
    (bind _turntimeline (Timeline|TurnTime PlayFromStart)
      (:Update
        (Variables|Default|SetTimer (Math|Conversions|ToInteger(Byte) (Utilities|String|ToString(Float) _turntimeline)))
        (if (Variables|/Game/Player/BP_Player.BP_Player_C|GetImDone (Variables|Default|GetPlayerRef))
          (Utilities|FlowControl|Delay 0.2)
          (Utilities|FlowControl|Sequence
            (:then_0
              (Timeline|TurnTime Stop))
            (:then_1
              (Default|EndMyTurn _playerref :!label _label_2)
              (bind _output_get (Variables|Default|SetCurrentEnemy 0))
              (Default|Attack (Utilities|Array|Get(acopy) (Variables|Default|GetEnemyList) _output_get) :!label _label_3)
              (Utilities|FlowControl|Delay 3.0)
              (Default|GoCasualPos (Utilities|Array|Get(acopy) (Variables|Default|GetEnemyList) _output_get))
              (Utilities|FlowControl|Delay 2.0)
              (if (== (Variables|Default|GetCurrentEnemy) (- (Utilities|Array|Length (Variables|Default|GetEnemyList)) 1))
                (CallFunction|UpdateOccupiedPos)
                (Variables|Default|SetCurrentEnemy 0)
                (goto _label)
                (else
                  (Variables|Default|SetCurrentEnemy (+ (Variables|Default|GetCurrentEnemy) 1))
                  (goto _label_3)))))))
      (:Finished
        (goto _label_2)))))

(event EventBeginPlay
  (bind _returnvalue (Game|SpawnActorfromClass "/Game/Player/BP_Player.BP_Player_C" (Math|Transform|MakeTransform "-300.000000,0.000000,20.000000" "0, 0, 0" "1,1,1") "Undefined" 0 0))
  (Variables|Default|SetPlayerRef _returnvalue)
  (for _index (range 0 (Variables|Default|GetEnemyToSpawn))
    (CallFunction|SpawnEnemy))
  (CallFunction|LoopStart))

(fn ConstructionScript)

(fn SpawnEnemy
  (bind _occupiedenemypos (Variables|Default|GetOccupiedEnemyPos))
  (if (== (Utilities|Array|Length _occupiedenemypos) 0)
    (LocalVariables|SetCellIndex (Math|Random|RandomIntegerinRange 0 24))
    (bind _returnvalue (Game|SpawnActorfromClass "/Game/Enemies/BP_Brawler.BP_Brawler_C" (Math|Transform|MakeTransform (Utilities|Array|Get(acopy) (.gridtransform (Variables|Default|GetEnemyGridRef)) (LocalVariables|GetCellIndex)) "0, 0, 0" "1,1,1") "Undefined" 0 0))
    (Utilities|Array|Add (Variables|Default|GetEnemyList) _returnvalue)
    (bind _newparam (Default|GetGridPos _returnvalue))
    (Utilities|Array|Add (Variables|Default|GetOccupiedEnemyPos) _newparam)
    (Variables|/Game/Enemies/BP_Enemy.BP_Enemy_C|SetEnemyNum _returnvalue (LocalVariables|Getcounter))
    (bind _result (Math|Integer|IncrementInt (LocalVariables|Getcounter))
      (:%20%20
        (LocalVariables|Setcounter _result)))
    (else
      (LocalVariables|SetCellIndex (Math|Random|RandomIntegerinRange 0 24) :!label _label)
      (bind _array_element (Utilities|Array|ForEachLoopwithBreak _occupiedenemypos)
        (:LoopBody
          (if (Math|Vector|Equal(Vector) (Utilities|Array|Get(acopy) (.gridposition (Variables|Default|GetEnemyGridRef)) (LocalVariables|GetCellIndex)) _array_element 0.1)
            (LocalVariables|SetCellOccupied true)
            (if (LocalVariables|GetCellOccupied) :!label _label_2
              (LocalVariables|SetCellOccupied false)
              (goto _label)
              (else
                (bind _returnvalue_2 (Game|SpawnActorfromClass "/Game/Enemies/BP_Brawler.BP_Brawler_C" (Math|Transform|MakeTransform (Utilities|Array|Get(acopy) (.gridtransform (Variables|Default|GetEnemyGridRef)) (LocalVariables|GetCellIndex)) "0, 0, 0" "1,1,1") "Undefined" 0 0))
                (Utilities|Array|Add (Variables|Default|GetEnemyList) _returnvalue_2)
                (bind _newparam_2 (Default|GetGridPos _returnvalue_2))
                (Utilities|Array|Add (Variables|Default|GetOccupiedEnemyPos) _newparam_2)
                (bind _result_2 (Math|Integer|IncrementInt (LocalVariables|Getcounter))
                  (:%20%20
                    (bind _output_get (LocalVariables|Setcounter _result_2))
                    (Variables|/Game/Enemies/BP_Enemy.BP_Enemy_C|SetEnemyNum _returnvalue_2 _output_get)))))))
        (:Completed
          (goto _label_2))))))

(fn ReFillEnemyArr
  (Utilities|Array|Clear (Variables|Default|GetEnemyList))
  (bind _outactors (Actor|GetAllActorsOfClass "/Game/Enemies/BP_Enemy.BP_Enemy_C"))
  (for _array_element _outactors
    (if (not (Variables|/Game/Enemies/BP_Enemy.BP_Enemy_C|GetIsDiing _array_element))
      (Utilities|Array|Add (Variables|Default|GetEnemyList) _array_element))))

(fn UpdateOccupiedPos
  (Utilities|Array|Clear (Variables|Default|GetOccupiedEnemyPos))
  (for _array_element (Variables|Default|GetEnemyList)
    (Utilities|Array|Add (Variables|Default|GetOccupiedEnemyPos) (Variables|/Game/Enemies/BP_Enemy.BP_Enemy_C|GetMyGridPos _array_element))))