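; BP_BrawlerBox is a short-lived enemy hazard that drops downward and damages the player on overlap.
; On BeginPlay it waits briefly, slides its root straight down with MoveComponentTo, then destroys itself after another short pause.
; Any actor overlap with exactly the BP_Player class calls that player's TakeDamage with a fixed amount, independently of the drop sequence.
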(event EventBeginPlay
  (bind _defaultsceneroot (Variables|Default|GetDefaultSceneRoot))
  (bind _returnvalue (Transformation|GetWorldLocation _defaultsceneroot))
  (Utilities|FlowControl|Delay 0.5)
  (Components|MoveComponentTo _defaultsceneroot (Math|Vector|MakeVector (.x _returnvalue) (.y _returnvalue) (- (.z _returnvalue) 3e+02)) (Transformation|GetWorldRotation _defaultsceneroot) false false 1.0 false)
  (Utilities|FlowControl|Delay 0.5)
  (Actor|DestroyActor))

(event Collision|EventActorBeginOverlap
  (params (OtherActor :type Actor%20Object%20Reference))
  (if (== (Utilities|GetClass OtherActor) "/Game/Player/BP_Player.BP_Player_C")
    (bind _asbp_player (Utilities|Casting|CastToBP_Player OtherActor))
    (Default|TakeDamage _asbp_player 2e+01)))

(fn ConstructionScript)