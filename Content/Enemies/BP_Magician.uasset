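; BP_Magician is a child enemy Blueprint whose attack fires a light bolt.
; Its Attack function calls Wait, then spawns BP_LightBolt at the mesh location with a fixed rotation, while BeginPlay and construction defer to the parent.
; Attack also holds disconnected, never-run leftovers for grid repositioning, lightning warnings at the player's cell, BrawlerBox spawns and a vulnerability count.
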(event EventBeginPlay
  (|CallParentFunction))

(fn ConstructionScript
  (|CallParentFunction))

(fn Attack
  (CallFunction|Wait)
  (Game|SpawnActorfromClass "/Game/Enemies/BP_LightBolt.BP_LightBolt_C" (Math|Transform|MakeTransform (Transformation|GetWorldLocation (Variables|Character|GetMesh)) "45.000000, 0, 0" "1,1,1") "Undefined" 0 0))