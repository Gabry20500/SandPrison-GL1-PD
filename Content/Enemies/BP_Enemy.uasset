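; Grid-based enemy actor with health, damage and a countdown-limited vulnerable state that doubles damage taken.
; Tick steps it toward destinations set by random-cell or return moves, then snaps and resolves its grid cell by location.
; TakeDamage updates the life widget; death awards the player AP by enemy count, has BP_GameManager_ refill its enemy array and destroys the actor.
; Attack only prints, and random-cell selection re-rolls separately for check, position and destination.
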(event Custom|Wait
  (Utilities|FlowControl|Delay 1.0))

(event EventTick
  (params (DeltaSeconds :type Float%20%28single-precision%29))
  (Utilities|FlowControl|Sequence
    (:then_0
      (if (Variables|Movement|GetCanMove)
        (Development|PrintString (Utilities|String|ToString(Float) (Variables|Default|GetHealth)) true true "(R=1.000000,G=0.000000,B=0.072754,A=1.000000)" 0.0)))
    (:then_1
      (if (Math|Vector|Equal(Vector) (Variables|Movement|GetCurrentLocation) (Variables|Movement|GetActualDestination) 1e+01)
        (Variables|Movement|SetCanMove false)
        (Transformation|SetWorldLocation (Variables|Default|GetDefaultSceneRoot) (Variables|Movement|GetActualDestination) false false)
        (CallFunction|UpdateGridPos)
        (else
          (bind _output_get (Variables|Movement|SetCurrentLocation (+ (Variables|Movement|GetCurrentLocation) (* (Variables|Movement|GetVelocity) (Variables|Movement|GetSpeed)))))
          (Transformation|SetWorldLocation (Variables|Default|GetDefaultSceneRoot) _output_get false false))))))

(event EventBeginPlay
  (bind _currentlocation (Variables|Movement|GetCurrentLocation))
  (bind _returnvalue (Actor|GetActorOfClass "/Game/BP_GameManager_.BP_GameManager__C"))
  (Variables|Default|SetGM_Ref _returnvalue)
  (CallFunction|UpdateGridPos)
  (bind _returnvalue_2 (Actor|GetActorOfClass "/Game/Player/BP_Player.BP_Player_C"))
  (Variables|Default|SetPlayerRef _returnvalue_2)
  (Variables|Movement|SetActualDestination _currentlocation)
  (Variables|Movement|SetPreviousLocation _currentlocation))

(fn ConstructionScript)

(fn GetHealth
  (return (Variables|Default|GetHealth)))

(fn GetDamage
  (return (Variables|Default|GetDamage)))

(fn GetGridPos
  (return (Variables|Movement|GetMyGridPos)))

(fn GetWorldTransform
  (return (Variables|Movement|GetCurrentLocation)))

(fn Attack
  (Development|PrintString "Attack" true true "(R=0.000000,G=0.660000,B=1.000000,A=1.000000)" 1.0))

(fn ReturntoPos
  (CallFunction|SetDestination (Variables|Movement|GetPreviousLocation))
  (Development|PrintString "Returning to pos")
  (Development|PrintString (Utilities|String|ToString(Integer) (Variables|Default|GetEnemyNum))))

(fn GoCasualPos
  (bind _returnvalue (Math|Random|RandomIntegerinRange 0 24))
  (bind _enemygridref (Variables|Default|GetEnemyGridRef))
  (bind _output (Utilities|Array|Get(acopy) _enemygridref))
  (bind _output_2 (Utilities|Array|Get(acopy) (.gridposition _output) _returnvalue))
  (LocalVariables|SetRandIndex _returnvalue :!label _label)
  (for _array_element (Variables|/Game/BP_GameManager_.BP_GameManager__C|GetOccupiedEnemyPos (Variables|Default|GetGM_Ref))
    (if (Math|Vector|Equal(Vector) _array_element _output_2 0.0001)
      (goto _label)))
  (Variables|Movement|SetMyGridPos _output_2)
  (CallFunction|SetDestination (Utilities|Array|Get(acopy) (.gridtransform _output) _returnvalue))
  (Default|UpdateOccupiedPos (Variables|Default|GetGM_Ref)))

(fn UpdateGridPos
  (bind _mesh (Variables|Default|GetMesh))
  (bind _returnvalue (Transformation|GetWorldLocation _mesh))
  (Variables|Movement|SetCurrentLocation (Transformation|GetWorldLocation (Variables|Default|GetDefaultSceneRoot)))
  (for _array_element (Variables|Default|GetEnemyGridRef)
    (for _index (range 0 (- (Utilities|Array|Length (.gridtransform _array_element)) 1))
      (if (Math|Vector|Equal(Vector) (Math|Vector|MakeVector (.x _returnvalue) (.y _returnvalue) 0.0) (Math|Vector|MakeVector (.x (Utilities|Array|Get(acopy) (.gridtransform _array_element) _index)) (.y (Utilities|Array|Get(acopy) (.gridtransform _array_element) _index)) 0.0) 3e+01)
        (bind _output_get (Variables|Movement|SetMyGridPos (Utilities|Array|Get(acopy) (.gridposition _array_element) _index)))
        (return _output_get)))))

(fn TakeDamage
  (params (DMG :type Float%20%28single-precision%29))
  (if (Variables|Default|GetisVulnerable)
    (Variables|Default|SetHealth (- (Variables|Default|GetHealth) (* 2 DMG)))
    (else
      (bind _output_get (Variables|Default|SetHealth (- (Variables|Default|GetHealth) DMG)))))
  (bind _asenemy_life_wg (Utilities|Casting|CastToEnemyLife_WG (UserInterface|GetWidget (Variables|Default|GetWidget))))
  (Progress|SetPercent (Variables|/Game/Player/UI/EnemyLife_UI/EnemyLife_WG.EnemyLife_WG_C|GetProgressBar_0 _asenemy_life_wg) (/ (Variables|Default|GetHealth) (Variables|Default|GetMaxHP)))
  (if (<= _output_get 0.0)
    (CallFunction|ReturnReward)
    (Variables|Default|SetIsDiing true)
    (Default|ReFillEnemyArr (Variables|Default|GetGM_Ref))
    (CallFunction|Wait)
    (Actor|DestroyActor)))

(fn SetDestination
  (params (Destination :type Vector))
  (Variables|Movement|SetActualDestination Destination)
  (Variables|Movement|SetVelocity (Math|Vector|Normalize (- (Variables|Movement|GetActualDestination) (Variables|Movement|GetCurrentLocation))))
  (Variables|Movement|SetCanMove true))

(fn ReturnReward
  (switch int (Utilities|Array|Length (Variables|/Game/BP_GameManager_.BP_GameManager__C|GetEnemyList (Variables|Default|GetGM_Ref)))
    (:1
      (Default|AddAp (Variables|Default|GetPlayerRef) 2))
    (:2
      (Default|AddAp (Variables|Default|GetPlayerRef) 3))
    (:3
      (Default|AddAp (Variables|Default|GetPlayerRef) 3))))

(fn VulnCount
  (Variables|Default|SetVulnerableCount (- (Variables|Default|GetVulnerableCount) 1))
  (if (== (Variables|Default|GetVulnerableCount) 0)
    (Variables|Default|SetisVulnerable false)))