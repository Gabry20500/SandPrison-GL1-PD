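; BP_LightBolt is an enemy lightning attack that targets the player's grid cell and damages the player on overlap.
; On BeginPlay it moves above that cell, re-samples the player's position, spawns a BP_WarningLighting marker, then descends onto it.
; It then hides, spawns BP_DamageLight tiles in a four-armed cross using stepped loops clipped to hard-coded arena bounds, and destroys itself.
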(event Custom|LightCross
  (bind _pglocation (Variables|Default|GetpgLocation))
  (Utilities|FlowControl|Sequence
    (:then_0
      (|UpperCross))
    (:then_1
      (|DownwardCross))
    (:then_2
      (Utilities|FlowControl|ForLoopwithBreak 0 4 :!label _label
        (:LoopBody
          (if (< (+ (.x (Variables|Default|GetpgLocation)) (Variables|Default|GetPlatformOffset)) -1.0)
            (Game|SpawnActorfromClass "/Game/Enemies/BP_DamageLight.BP_DamageLight_C" (Math|Transform|MakeTransform (Math|Vector|MakeVector (+ (.x _pglocation) (Variables|Default|GetPlatformOffset)) (.y _pglocation) 14.0) "0, 0, 0" "1.000000,1,0.010000") "Undefined" 0 0)
            (Variables|Default|SetPlatformOffset (+ (Variables|Default|GetPlatformOffset) 1e+02))
            (else
              (Variables|Default|SetPlatformOffset 1e+02)
              (goto _label Break))))))
    (:then_3
      (|LeftCross))))

(event EventBeginPlay
  (bind _defaultsceneroot (Variables|Default|GetDefaultSceneRoot))
  (bind _returnvalue (Actor|GetActorOfClass "/Game/Player/BP_Player.BP_Player_C"))
  (bind _output_get (Variables|Default|SetpgRef _returnvalue))
  (bind _output_get_2 (Variables|Default|SetpgLocation (Math|Vector|MakeVector (- (* (.x (Variables|/Game/Player/BP_Player.BP_Player_C|GetCurrentGridPos _output_get)) 1e+02) 1e+02) (* (.y (Variables|/Game/Player/BP_Player.BP_Player_C|GetCurrentGridPos _output_get)) 1e+02) 0.0)))
  (Components|MoveComponentTo _defaultsceneroot (Math|Vector|MakeVector (.x _output_get_2) (.y _output_get_2) 6e+02) (Transformation|GetWorldRotation _defaultsceneroot) false false 1.0 false)
  (Utilities|FlowControl|Delay 0.2)
  (Variables|Default|SetpgLocation (Math|Vector|MakeVector (- (* (.x (Variables|/Game/Player/BP_Player.BP_Player_C|GetCurrentGridPos (Variables|Default|GetpgRef))) 1e+02) 1e+02) (* (.y (Variables|/Game/Player/BP_Player.BP_Player_C|GetCurrentGridPos (Variables|Default|GetpgRef))) 1e+02) 0.0))
  (Game|SpawnActorfromClass "/Game/Enemies/BP_WarningLighting.BP_WarningLighting_C" (Math|Transform|MakeTransform (Math|Vector|MakeVector (- (* (.x (Variables|/Game/Player/BP_Player.BP_Player_C|GetCurrentGridPos (Variables|Default|GetpgRef))) 1e+02) 1e+02) (* (.y (Variables|/Game/Player/BP_Player.BP_Player_C|GetCurrentGridPos (Variables|Default|GetpgRef))) 1e+02) 14.0) "0, 0, 0" "1.000000,1,0.010000") "Undefined" 0 0)
  (Components|MoveComponentTo (Variables|Default|GetDefaultSceneRoot) (Math|Vector|MakeVector (.x (Variables|Default|GetpgLocation)) (.y (Variables|Default|GetpgLocation)) 0.0) "180.000000, 0, 0" false false 0.8 false)
  (Utilities|FlowControl|Delay 0.1)
  ;[1 1 1] Comment
  (Utilities|FlowControl|Sequence
    (:then_0
      (Rendering|SetVisibility (Variables|Default|GetDefaultSceneRoot self) false true))
    (:then_1
      (CallFunction|LightCross))
    (:then_2
      (Actor|DestroyActor))))

(event Collision|EventActorBeginOverlap
  (params (OtherActor :type Actor%20Object%20Reference))
  (if (== (Utilities|GetClass OtherActor) "/Game/Player/BP_Player.BP_Player_C")
    (bind _asbp_player (Utilities|Casting|CastToBP_Player OtherActor))
    (Default|TakeDamage _asbp_player 15.0)))

(fn ConstructionScript)