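; Turn-based game manager that spawns the player and a set of enemies, then starts the turn cycle.
; SpawnEnemy places each enemy on a random grid cell, re-rolling against recorded occupied positions.
; LoopStart sets the player's turn and plays the TurnTime timeline inside a fixed for loop, which does not wait for it to finish.
; When the timeline finishes, the player's turn ends and every enemy attacks and repositions.
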(event Custom|LoopStart
  (bind _playerref (Variables|Default|GetPlayerRef))
  (for _index (range 0 99)
    (Variables|/Game/Player/BP_Player.BP_Player_C|SetIsMyTurn? _playerref true)
    (bind _turntimeline (Timeline|TurnTime Play)
      (:Update
        (Development|PrintString (Utilities|String|ToString(Integer) (Math|Conversions|ToInteger(Byte) (Utilities|String|ToString(Float) _turntimeline))) true true "(R=0.908333,G=0.024228,B=0.017000,A=1.000000)" 0.0))
      (:Finished
        (Default|EndMyTurn _playerref)
        (for _array_element (Variables|Default|GetEnemyList)
          (Default|Attack _array_element)
          (Default|ReturntoPos _array_element)
          (Default|GoCasualPos _array_element))))))

(event EventBeginPlay
  (bind _returnvalue (Game|SpawnActorfromClass "/Game/Player/BP_Player.BP_Player_C" (Math|Transform|MakeTransform "-300.000000,0.000000,20.000000" "0, 0, 0" "1,1,1") "Undefined" 0 0))
  (Variables|Default|SetPlayerRef _returnvalue)
  (for _index (range 0 (Variables|Default|GetEnemyToSpawn))
    (CallFunction|SpawnEnemy))
  (CallFunction|LoopStart))

(fn ConstructionScript)

(fn SpawnEnemy
  (bind _occupiedenemypos (Variables|Default|GetOccupiedEnemyPos))
  (if (== (Utilities|Array|Length _occupiedenemypos) 0)
    (LocalVariables|SetCellIndex (Math|Random|RandomIntegerinRange 0 24))
    (bind _returnvalue (Game|SpawnActorfromClass "/Game/Enemies/BP_Enemy.BP_Enemy_C" (Math|Transform|MakeTransform (Utilities|Array|Get(acopy) (.gridtransform (Variables|Default|GetEnemyGridRef)) (LocalVariables|GetCellIndex)) "0, 0, 0" "1,1,1") "Undefined" 0 0))
    (Utilities|Array|Add (Variables|Default|GetEnemyList) _returnvalue)
    (bind _newparam (Default|GetGridPos _returnvalue))
    (Utilities|Array|Add (Variables|Default|GetOccupiedEnemyPos) _newparam)
    (else
      (LocalVariables|SetCellIndex (Math|Random|RandomIntegerinRange 0 24) :!label _label)
      (bind _array_element (Utilities|Array|ForEachLoopwithBreak _occupiedenemypos)
        (:LoopBody
          (if (Math|Vector|Equal(Vector) (Utilities|Array|Get(acopy) (.gridposition (Variables|Default|GetEnemyGridRef)) (LocalVariables|GetCellIndex)) _array_element 0.1)
            (LocalVariables|SetCellOccupied true)))
        (:Completed
          (if (LocalVariables|GetCellOccupied)
            (goto _label)
            (else
              (bind _returnvalue_2 (Game|SpawnActorfromClass "/Game/Enemies/BP_Enemy.BP_Enemy_C" (Math|Transform|MakeTransform (Utilities|Array|Get(acopy) (.gridtransform (Variables|Default|GetEnemyGridRef)) (LocalVariables|GetCellIndex)) "0, 0, 0" "1,1,1") "Undefined" 0 0))
              (Utilities|Array|Add (Variables|Default|GetEnemyList) _returnvalue_2)
              (bind _newparam_2 (Default|GetGridPos _returnvalue_2))
              (Utilities|Array|Add (Variables|Default|GetOccupiedEnemyPos) _newparam_2))))))))